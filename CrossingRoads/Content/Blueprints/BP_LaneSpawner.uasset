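; BP_LaneSpawner builds and recycles a chain of BP_Lane segments, starting just below the player pawn.
; On BeginPlay it clears existing lanes, then chains an initial run, each placed at the previous lane's SpawnPoint.
; SpawnLane gives each lane a back-reference and random SetLane variant, narrower for the first two, and retires the oldest beyond MaxLanes.
; SpawnLaneAtSpawnPoint extends the chain from the newest lane.
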(event EventBeginPlay
  (Variables|Default|SetRand (Math|Random|RandomIntegerinRange 0 6))
  (CallFunction|SpawnInitialLanes))

(event EventTick
  (params (DeltaSeconds :type Float%20%28single-precision%29)))

(fn ConstructionScript)

(fn SpawnInitialLanes
  (Utilities|FlowControl|Sequence
    (:then_0
      (bind _outactors (Actor|GetAllActorsOfClass "/Game/Blueprints/BP_Lane.BP_Lane_C"))
      (for _array_element _outactors
        (Actor|DestroyActor _array_element)))
    (:then_1
      (for _index (range 0 0)
        (Utilities|IsValid (Variables|Default|GetNewestLane)
          (:Is%20Valid
            (CallFunction|SpawnLaneatSpawnPoint))
          (:Is%20Not%20Valid
            (for _index_2 (range 0 8)
              (if (== _index_2 0)
                (CallFunction|SpawnLane (- (Transformation|GetActorLocation (Game|Player|GetPlayerPawn 0)) "0, 0,40.000000"))
                (Variables|/Game/Blueprints/BP_Lane.BP_Lane_C|SetisSpawnTriggered (Utilities|Array|Get(acopy) (Variables|Default|GetarrayOfLanes)) false)
                (else
                  (CallFunction|SpawnLane (Transformation|GetWorldLocation (Variables|/Game/Blueprints/BP_Lane.BP_Lane_C|GetSpawnPoint (Variables|Default|GetNewestLane))))
                  (Variables|/Game/Blueprints/BP_Lane.BP_Lane_C|SetisSpawnTriggered (Utilities|Array|Get(acopy) (Variables|Default|GetarrayOfLanes) 1) false))))))))))

(fn SpawnLaneatSpawnPoint
  (CallFunction|SpawnLane (Transformation|GetWorldLocation (Variables|/Game/Blueprints/BP_Lane.BP_Lane_C|GetSpawnPoint (Variables|Default|GetNewestLane)))))

(fn SpawnLane
  (params (SpawnLocation :type Vector))
  (bind _arrayoflanes (Variables|Default|GetarrayOfLanes))
  (bind _returnvalue (Game|SpawnActorfromClass "/Game/Blueprints/BP_Lane.BP_Lane_C" (Math|Transform|MakeTransform SpawnLocation "0, 0, 0" "1,1,1") "Undefined" 0 0))
  (if (<= (Utilities|Array|Length _arrayoflanes) (Variables|Default|GetmaxLanes))
    _
    (else
      (Default|DestroyLane (Utilities|Array|Get(acopy) _arrayoflanes))
      (Utilities|Array|RemoveIndex _arrayoflanes)))
  (bind _output_get (Variables|Default|SetNewestLane _returnvalue))
  (Variables|/Game/Blueprints/BP_Lane.BP_Lane_C|SetLaneSpawner _output_get self)
  (if (<= (Utilities|Array|Length (Variables|Default|GetarrayOfLanes)) 1)
    (Default|SetLane _output_get (Math|Random|RandomIntegerinRange 0 1))
    (Utilities|Array|Add (Variables|Default|GetarrayOfLanes) (Variables|Default|GetNewestLane))
    (else
      (Default|SetLane _output_get (Math|Random|RandomIntegerinRange 0 6))
      (Utilities|Array|Add (Variables|Default|GetarrayOfLanes) (Variables|Default|GetNewestLane)))))
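; Lane object for a Crossy Road-style game that becomes a car, river float or grass prop, despite its spawner name.
; SetCar, SetRiver and SetGrassMisc set the Type and pick a random mesh, including a collectible coin among grass props.
; Tick moves cars and floats at random speeds until a Y limit destroys them.
; Chicken overlap either squashes it and shows the restart HUD, or collects coins into GameModeCrossy's count.
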(event EventBeginPlay
  (Variables|Default|SetrandSpeed (Math|Random|RandomFloatinRange 2e+02 4.5e+02)))

(event Collision|EventActorBeginOverlap
  (params (OtherActor :type Actor%20Object%20Reference))
  ;[1 1 1] VehicleSquash
  (bind _aschicken (Utilities|Casting|CastToChicken OtherActor))
  (if (== (Variables|Default|GetType) 0)
    (Class|Actor|AddActorLocalTransform _aschicken (Math|Transform|MakeTransform "0, 0, 0" "0, 0, 0" "1,1,0.100000") false false)
    (Pawn|Components|CharacterMovement|DisableMovement (Variables|/Script/Engine.Character|GetCharacterMovement _aschicken))
    (CallFunction|ResetGame)
    (else
      ;[1 1 1] CoinCollect
      (if (== "/Game/Assets/Misc/coin_Coin.coin_Coin" (Variables|/Script/Engine.StaticMeshComponent|GetStaticMesh (Variables|Default|GetVehicle)))
        (Actor|DestroyActor)
        (bind _asgame_mode_crossy (Utilities|Casting|CastToGameModeCrossy (Game|GetGameMode)))
        (Variables|/Game/Blueprints/GameMode/GameModeCrossy.GameModeCrossy_C|SetCoinCount _asgame_mode_crossy (+ (Variables|/Game/Blueprints/GameMode/GameModeCrossy.GameModeCrossy_C|GetCoinCount _asgame_mode_crossy) 1))))))

(event EventTick
  (params (DeltaSeconds :type Float%20%28single-precision%29))
  (bind _type (Variables|Default|GetType))
  ;[1 1 1] VehicleMove/Destroy
  (if (or (== _type 0) (== _type 1))
    (if (>= (.y (Transformation|GetActorLocation)) 1.08e+03)
      (Actor|DestroyActor)
      (else
        (Transformation|AddActorLocalOffset (Math|Vector|MakeVector 0.0 (* DeltaSeconds (Variables|Default|GetrandSpeed)) 0.0) false false)))))

(fn ConstructionScript)

(fn DestroyCar
  (Actor|DestroyActor))

(fn Train)

(fn SetCar
  (bind _vehicle (Variables|Default|GetVehicle))
  (Variables|Default|SetType 0)
  (switch int (Math|Random|RandomIntegerinRange 0 9)
    (:0
      (Components|StaticMesh|SetStaticMesh _vehicle "/Game/Assets/Vehicles/car_small.car_small"))
    (:1
      (Components|StaticMesh|SetStaticMesh _vehicle "/Game/Assets/Vehicles/pizza_car_Untitled.pizza_car_Untitled"))
    (:2
      (Components|StaticMesh|SetStaticMesh _vehicle "/Game/Assets/Vehicles/policeCar_policeCar.policeCar_policeCar"))
    (:3
      (Components|StaticMesh|SetStaticMesh _vehicle "/Game/Assets/Vehicles/policeCar_policeCar.policeCar_policeCar"))
    (:4
      (Components|StaticMesh|SetStaticMesh _vehicle "/Game/Assets/Vehicles/taxi_taxi.taxi_taxi"))
    (:5
      (Components|StaticMesh|SetStaticMesh _vehicle "/Game/Assets/Vehicles/Amazon_Truck.Amazon_Truck"))
    (:6
      (Components|StaticMesh|SetStaticMesh _vehicle "/Game/Assets/Vehicles/FedExTruck.FedExTruck"))
    (:7
      (Components|StaticMesh|SetStaticMesh _vehicle "/Game/Assets/Vehicles/upsTruck_Untitled.upsTruck_Untitled"))
    (:8
      (Components|StaticMesh|SetStaticMesh _vehicle "/Game/Assets/Vehicles/USPStruck_Untitled.USPStruck_Untitled"))
    (:9
      (Components|StaticMesh|SetStaticMesh _vehicle "/Game/Assets/Vehicles/corvette.corvette"))))

(fn SetRiver
  (bind _vehicle (Variables|Default|GetVehicle))
  (bind _vehicle_2 (Variables|Default|GetVehicle))
  (Variables|Default|SetType 1)
  (switch int (Math|Random|RandomIntegerinRange 0 3)
    (:0
      (Components|StaticMesh|SetStaticMesh _vehicle "/Game/Assets/Misc/large_log_Untitled.large_log_Untitled"))
    (:1
      (Components|StaticMesh|SetStaticMesh _vehicle "/Game/Assets/Misc/medium_log_Untitled.medium_log_Untitled"))
    (:2
      (Components|StaticMesh|SetStaticMesh _vehicle_2 "/Game/Assets/Misc/small_log_Untitled.small_log_Untitled"))
    (:3
      (Components|StaticMesh|SetStaticMesh _vehicle_2 "/Game/Assets/Misc/lilypad_lilypad.lilypad_lilypad")))
  (Variables|Default|SetrandSpeed (Math|Random|RandomFloatinRange 1e+02 2.5e+02)))

(fn SetGrassMisc
  (bind _vehicle (Variables|Default|GetVehicle))
  (Variables|Default|SetType 2)
  (switch int (Math|Random|RandomIntegerinRange 0 7)
    (:0
      (Components|StaticMesh|SetStaticMesh _vehicle "/Game/Assets/Misc/italian_tree_Italian_Tree.italian_tree_Italian_Tree"))
    (:1
      (Components|StaticMesh|SetStaticMesh _vehicle "/Game/Assets/Misc/large_tree_Untitled.large_tree_Untitled"))
    (:2
      (Components|StaticMesh|SetStaticMesh _vehicle "/Game/Assets/Misc/medium_tree_Untitled.medium_tree_Untitled"))
    (:3
      (Components|StaticMesh|SetStaticMesh _vehicle "/Game/Assets/Misc/med_bush_Untitled.med_bush_Untitled"))
    (:4
      (Components|StaticMesh|SetStaticMesh _vehicle "/Game/Assets/Misc/small_bush.small_bush"))
    (:5
      (Components|StaticMesh|SetStaticMesh _vehicle "/Game/Assets/Misc/rock_Rock.rock_Rock"))
    (:6
      (Components|StaticMesh|SetStaticMesh _vehicle "/Game/Assets/Misc/palm_palm_basic.palm_palm_basic"))
    (:7
      (Components|StaticMesh|SetStaticMesh _vehicle "/Game/Assets/Misc/coin_Coin.coin_Coin"))))

(fn ResetGame
  (bind _returnvalue (UserInterface|CreateWidget "/Game/Widget/RestartHUD.RestartHUD_C"))
  (UserInterface|Viewport|AddtoViewport _returnvalue 0))
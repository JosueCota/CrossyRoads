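; One lane of a Crossy Road-style game, built from thirteen mesh tiles that SetLane re-skins as grass, railroad, river or road.
; Roads and rivers periodically spawn BP_VehicleSpawner actors at random intervals, while grass scatters prop spawners tracked for cleanup in DestroyLane.
; The Chicken's first trigger overlap asks LaneSpawner for another lane and increments score.
; River contact plays a splash and Timeline sink, then disables movement and shows RestartHUD.
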(event OnComponentBeginOverlap(LaneTrigger)
  (params (OverlappedComponent :type Primitive%20Component%20Object%20Reference) (OtherActor :type Actor%20Object%20Reference) (OtherComp :type Primitive%20Component%20Object%20Reference) (OtherBodyIndex :type Integer) (bFromSweep :type Boolean) (SweepResult :type Hit%20Result%20Structure%20%28by%20ref%29))
  ;[1 1 1] LaneSpawning
  (if (not (Variables|Default|GetisSpawnTriggered))
    (Utilities|Casting|CastToChicken OtherActor)
    (Default|SpawnLaneatSpawnPoint (Variables|Default|GetLaneSpawner))
    (Variables|Default|SetisSpawnTriggered true)
    (bind _asgame_mode_crossy (Utilities|Casting|CastToGameModeCrossy (Game|GetGameMode)))
    (Variables|/Game/Blueprints/GameMode/GameModeCrossy.GameModeCrossy_C|SetScoreCount _asgame_mode_crossy (+ (Variables|/Game/Blueprints/GameMode/GameModeCrossy.GameModeCrossy_C|GetScoreCount _asgame_mode_crossy) 1))))

(event OnComponentBeginOverlap(Watercheck)
  (params (OverlappedComponent :type Primitive%20Component%20Object%20Reference) (OtherActor :type Actor%20Object%20Reference) (OtherComp :type Primitive%20Component%20Object%20Reference) (OtherBodyIndex :type Integer) (bFromSweep :type Boolean) (SweepResult :type Hit%20Result%20Structure%20%28by%20ref%29))
  ;[1 1 1] WaterSplash
  (Variables|Default|SetChickStart (Transformation|GetActorLocation OtherActor))
  (if (== (Variables|Default|GetLaneType) 1)
    (bind _aschicken (Utilities|Casting|CastToChicken OtherActor))
    (Effects|SpawnEmitteratLocation "/Game/Material/P_Water.P_Water" (Transformation|GetActorLocation OtherActor))
    (bind _newtrack_0 (Timeline|Sink Play)
      (:Update
        (Transformation|SetActorLocation OtherActor (Math|Interpolation|Ease "Linear" _newtrack_0 (Variables|Default|GetChickStart) (- (Variables|Default|GetChickStart) "0, 0,50.000000")) false false))
      (:Finished
        (Pawn|Components|CharacterMovement|DisableMovement (Variables|/Script/Engine.Character|GetCharacterMovement _aschicken))
        (CallFunction|ResetGame)))))

(event Custom|CanSpawn
  ;[1 1 1] VehicleSpawning
  (Utilities|FlowControl|DoOnce false :!label _label
    (:Completed
      (Variables|Default|SetSpawnable false)
      (Utilities|FlowControl|Delay (Math|Random|RandomFloatinRange 2.0 4.0))
      (Variables|Default|SetSpawnable true)
      (goto _label Reset))))

(event Custom|VehicleTick
  ;[1 1 1] VehicleSpawning
  (CallFunction|VehicleSpawn)
  (CallFunction|CanSpawn))

(event EventTick
  (params (DeltaSeconds :type Float%20%28single-precision%29))
  (bind _lanetype (Variables|Default|GetLaneType))
  ;[1 1 1] VehicleSpawning
  (if (or (== _lanetype 0) (== _lanetype 1))
    (if (Variables|Default|GetSpawnable)
      (CallFunction|VehicleTick))))

(fn ConstructionScript
  (Utilities|Array|Add (Variables|Default|GetLaneArrayContainer) (Variables|Default|GetLane1))
  (Utilities|Array|Add (Variables|Default|GetLaneArrayContainer) (Variables|Default|GetLane2))
  (Utilities|Array|Add (Variables|Default|GetLaneArrayContainer) (Variables|Default|GetLane3))
  (Utilities|Array|Add (Variables|Default|GetLaneArrayContainer) (Variables|Default|GetLane4))
  (Utilities|Array|Add (Variables|Default|GetLaneArrayContainer) (Variables|Default|GetLane5))
  (Utilities|Array|Add (Variables|Default|GetLaneArrayContainer) (Variables|Default|GetLane6))
  (Utilities|Array|Add (Variables|Default|GetLaneArrayContainer) (Variables|Default|GetLane7))
  (Utilities|Array|Add (Variables|Default|GetLaneArrayContainer) (Variables|Default|GetLane8))
  (Utilities|Array|Add (Variables|Default|GetLaneArrayContainer) (Variables|Default|GetLane9))
  (Utilities|Array|Add (Variables|Default|GetLaneArrayContainer) (Variables|Default|GetLane10))
  (Utilities|Array|Add (Variables|Default|GetLaneArrayContainer) (Variables|Default|GetLane11))
  (Utilities|Array|Add (Variables|Default|GetLaneArrayContainer) (Variables|Default|GetLane12))
  (Utilities|Array|Add (Variables|Default|GetLaneArrayContainer) (Variables|Default|GetLane13)))

(fn SetLane
  (params (Rand :type Integer))
  (switch int Rand
    (:0
      (CallFunction|GrassLanes :!label _label))
    (:1
      (goto _label))
    (:2
      (CallFunction|TrainLane))
    (:3
      (CallFunction|RiverLanes :!label _label_2))
    (:4
      (goto _label_2))
    (:5
      (CallFunction|RoadLane))
    (:6
      (CallFunction|MarkedRoadLane))))

(fn GrassLanes
  (bind _lanearraycontainer (Variables|Default|GetLaneArrayContainer))
  (bind _lanearraycontainer_2 (Variables|Default|GetLaneArrayContainer))
  (Variables|Default|SetLaneType 2)
  (if (== (Math|Random|RandomIntegerinRange 0 1) 0)
    (for _index (range 0 (- (Utilities|Array|Length _lanearraycontainer) 1))
      (Components|StaticMesh|SetStaticMesh (Utilities|Array|Get(acopy) _lanearraycontainer _index) "/Game/Assets/Misc/lightgrass_Untitled.lightgrass_Untitled")
      (if (and (!= (Utilities|Array|Length (Variables|/Game/Blueprints/BP_LaneSpawner.BP_LaneSpawner_C|GetarrayOfLanes (Variables|Default|GetLaneSpawner))) 0) (>= (Math|Random|RandomFloatinRange 0.0 1.0) 0.8))
        (Variables|Default|SetSpawnLocation (- (Transformation|GetWorldLocation (Utilities|Array|Get(acopy) _lanearraycontainer _index)) "0, 0,-20.000000"))
        (CallFunction|VehicleSpawn)))
    (else
      (for _index_2 (range 0 (- (Utilities|Array|Length _lanearraycontainer_2) 1))
        (Components|StaticMesh|SetStaticMesh (Utilities|Array|Get(acopy) _lanearraycontainer_2 _index_2) "/Game/Assets/Misc/darkgrass_Untitled.darkgrass_Untitled")
        (if (and (!= (Utilities|Array|Length (Variables|/Game/Blueprints/BP_LaneSpawner.BP_LaneSpawner_C|GetarrayOfLanes (Variables|Default|GetLaneSpawner))) 0) (>= (Math|Random|RandomFloatinRange 0.0 1.0) 0.8))
          (Variables|Default|SetSpawnLocation (- (Transformation|GetWorldLocation (Utilities|Array|Get(acopy) _lanearraycontainer_2 _index_2)) "0, 0,-20.000000"))
          (CallFunction|VehicleSpawn))))))

(fn TrainLane
  (bind _lanearraycontainer (Variables|Default|GetLaneArrayContainer))
  (for _index (range 0 (- (Utilities|Array|Length _lanearraycontainer) 1))
    (Components|StaticMesh|SetStaticMesh (Utilities|Array|Get(acopy) _lanearraycontainer _index) "/Game/Assets/Misc/railroad_Untitled.railroad_Untitled"))
  (Variables|Default|SetLaneType 3))

(fn RiverLanes
  (bind _lanearraycontainer (Variables|Default|GetLaneArrayContainer))
  (bind _lanearraycontainer_2 (Variables|Default|GetLaneArrayContainer))
  (if (== (Math|Random|RandomIntegerinRange 0 1) 0)
    (for _index (range 0 (- (Utilities|Array|Length _lanearraycontainer) 1))
      (Components|StaticMesh|SetStaticMesh (Utilities|Array|Get(acopy) _lanearraycontainer _index) "/Game/Assets/Misc/light_river_Untitled.light_river_Untitled"))
    (else
      (for _index_2 (range 0 (- (Utilities|Array|Length _lanearraycontainer_2) 1))
        (Components|StaticMesh|SetStaticMesh (Utilities|Array|Get(acopy) _lanearraycontainer_2 _index_2) "/Game/Assets/Misc/dark_river_Untitled.dark_river_Untitled"))))
  (Variables|Default|SetLaneType 1))

(fn RoadLane
  (bind _lanearraycontainer (Variables|Default|GetLaneArrayContainer))
  (for _index (range 0 (- (Utilities|Array|Length _lanearraycontainer) 1))
    (Components|StaticMesh|SetStaticMesh (Utilities|Array|Get(acopy) _lanearraycontainer _index) "/Game/Assets/Misc/unmarkedRoad.unmarkedRoad"))
  (Variables|Default|SetLaneType 0))

(fn MarkedRoadLane
  (bind _lanearraycontainer (Variables|Default|GetLaneArrayContainer))
  (for _index (range 0 (- (Utilities|Array|Length _lanearraycontainer) 1))
    (if (== (Math|Integer|%(Integer) _index 2) 0)
      (Components|StaticMesh|SetStaticMesh (Utilities|Array|Get(acopy) _lanearraycontainer _index) "/Game/Assets/Misc/sidemarkedRoad_Untitled.sidemarkedRoad_Untitled")
      (else
        (Components|StaticMesh|SetStaticMesh (Utilities|Array|Get(acopy) _lanearraycontainer _index) "/Game/Assets/Misc/unmarkedRoad.unmarkedRoad"))))
  (Variables|Default|SetLaneType 0))

(fn DestroyLane
  (bind _miscitems (Variables|Default|GetMiscItems))
  (if (== (Variables|Default|GetLaneType) 2)
    (for _index (range 0 (- (Utilities|Array|Length _miscitems) 1))
      (Actor|DestroyActor (Utilities|Array|Get(acopy) _miscitems _index))))
  (Actor|DestroyActor))

(fn VehicleSpawn
  (switch int (Variables|Default|GetLaneType)
    (:0
      (bind _returnvalue (Game|SpawnActorfromClass "/Game/Blueprints/BP_VehicleSpawner.BP_VehicleSpawner_C" (Math|Transform|MakeTransform (Transformation|GetWorldLocation (Variables|Default|GetVehicleSpawnPoint)) "0, 0, 0" "1,1,1") "Undefined" 0 0))
      (Default|SetCar _returnvalue))
    (:1
      (bind _returnvalue_2 (Game|SpawnActorfromClass "/Game/Blueprints/BP_VehicleSpawner.BP_VehicleSpawner_C" (Math|Transform|MakeTransform (Transformation|GetWorldLocation (Variables|Default|GetVehicleSpawnPoint)) "0, 0, 0" "1,1,1") "Undefined" 0 0))
      (Default|SetRiver _returnvalue_2))
    (:2
      (bind _returnvalue_3 (Game|SpawnActorfromClass "/Game/Blueprints/BP_VehicleSpawner.BP_VehicleSpawner_C" (Math|Transform|MakeTransform (Variables|Default|GetSpawnLocation) "0, 0, 0" "1,1,1") "Undefined" 0 0))
      (Default|SetGrassMisc _returnvalue_3)
      (Utilities|Array|Add (Variables|Default|GetMiscItems) _returnvalue_3))))

(fn ResetGame
  (bind _returnvalue (UserInterface|CreateWidget "/Game/Widget/RestartHUD.RestartHUD_C"))
  (UserInterface|Viewport|AddtoViewport _returnvalue 0))
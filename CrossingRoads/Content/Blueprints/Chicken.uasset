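; Player-controlled chicken Character that moves in short hops along the world X and Y axes.
; Forward and right axis input past a deadzone calls LaunchCharacter for each hop, while a timeline lerps the mesh to face the hop direction.
; A DoOnce-guarded cooldown briefly clears Canmove to space out hops.
; Turn and LookUp inputs drive controller yaw and pitch, independent of hop direction.
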(event Custom|MoveCooldown
  ;[1 1 1] MovementCooldown
  (Utilities|FlowControl|DoOnce false :!label _label
    (:Completed
      (Variables|Default|Setcanmove false)
      (Utilities|FlowControl|Delay 0.48)
      (Variables|Default|Setcanmove true)
      (goto _label Reset))))

(event Input|AxisEvents|InputAxisTurn
  (params (AxisValue :type Float%20%28single-precision%29))
  (Pawn|Input|AddControllerYawInput AxisValue))

(event Input|AxisEvents|InputAxisLookUp
  (params (AxisValue :type Float%20%28single-precision%29))
  (Pawn|Input|AddControllerPitchInput AxisValue))

(event Input|AxisEvents|InputAxisMoveForward
  (params (AxisValue :type Float%20%28single-precision%29))
  (bind _mesh (Variables|Character|GetMesh))
  (bind _mesh_2 (Variables|Character|GetMesh))
  ;[1 1 1] MoveForwardJump
  (if (and (> (Math|Float|Absolute(Float) AxisValue) 0.3) (Variables|Default|Getcanmove))
    (CallFunction|MoveCooldown)
    (Character|LaunchCharacter (Math|Vector|MakeVector (* AxisValue 2e+02) 0.0 2.2e+02) true true)
    ;[1 1 1] Character Rotation
    (if (> AxisValue 0.3)
      (bind _newtrack_0 (Timeline|Timeline_0 PlayFromStart)
        (:Update
          (Transformation|SetWorldRotation _mesh (Math|Rotator|Lerp(Rotator) (Transformation|GetWorldRotation _mesh) "0,90.000000, 0" _newtrack_0 true) false false)))
      (else
        (bind _newtrack_0_2 (Timeline|Timeline_1 PlayFromStart)
          (:Update
            (Transformation|SetWorldRotation _mesh_2 (Math|Rotator|Lerp(Rotator) (Transformation|GetWorldRotation _mesh_2) "0,-90.000000, 0" _newtrack_0_2 true) false false)))))))

(event Input|AxisEvents|InputAxisMoveRight
  (params (AxisValue :type Float%20%28single-precision%29))
  (bind _mesh (Variables|Character|GetMesh))
  (bind _mesh_2 (Variables|Character|GetMesh))
  ;[1 1 1] MoveRightJump
  (if (and (> (Math|Float|Absolute(Float) AxisValue) 0.3) (Variables|Default|Getcanmove))
    (CallFunction|MoveCooldown)
    (Character|LaunchCharacter (Math|Vector|MakeVector 0.0 (* AxisValue 2.2e+02) 2.2e+02) true true)
    ;[1 1 1] Character Rotation
    (if (> AxisValue 0.3)
      (bind _newtrack_0 (Timeline|Timeline_2 PlayFromStart)
        (:Update
          (Transformation|SetWorldRotation _mesh_2 (Math|Rotator|Lerp(Rotator) (Transformation|GetWorldRotation _mesh_2) "0,-180.000000, 0" _newtrack_0 true) false false)))
      (else
        (bind _newtrack_0_2 (Timeline|Timeline_3 PlayFromStart)
          (:Update
            (Transformation|SetWorldRotation _mesh (Math|Rotator|Lerp(Rotator) (Transformation|GetWorldRotation _mesh) "0, 0, 0" _newtrack_0_2 true) false false)))))))

(fn ConstructionScript)